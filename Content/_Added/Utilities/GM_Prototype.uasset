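; Prototype game mode that registers each joining player's character and gives them their own HUD.
; On new player start, it stores the player character in the ACGameLogic pilot list, indexed by controller ID.
; It then adds a W_HUD to that player's screen and stores its thruster bar in a parallel list.
; Two getter functions return a player's pilot or mech thrust bar by index.
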(event EventHandleStartingNewPlayer
  (params (NewPlayer :type Player%20Controller%20Object%20Reference))
  (bind _returnvalue (Class|GameplayStatics|GetPlayerControllerID NewPlayer))
  (|CallParentFunction NewPlayer)
  (Utilities|Array|SetArrayElem (Variables|/Game/_Added/Utilities/AC_GameLogic.AC_GameLogic_C|GetPlayerPilotList (Variables|Default|GetAC_GameLogic)) _returnvalue (Game|GetPlayerCharacter _returnvalue) true)
  (bind _returnvalue_2 (UserInterface|CreateWidget "/Game/_Added/UI/W_HUD.W_HUD_C" NewPlayer))
  (UserInterface|Viewport|AddtoPlayerScreen _returnvalue_2)
  (Utilities|Array|SetArrayElem (Variables|/Game/_Added/Utilities/AC_GameLogic.AC_GameLogic_C|GetPlayerThrusterList (Variables|Default|GetAC_GameLogic)) (Class|GameplayStatics|GetPlayerControllerID NewPlayer) (Variables|/Game/_Added/UI/W_HUD.W_HUD_C|GetThrusterBar _returnvalue_2) true))

(fn ConstructionScript)

(fn GetPlayerMechThrustBar
  (params (Index :type Integer))
  (return (Utilities|Array|Get(acopy) (Variables|/Game/_Added/Utilities/AC_GameLogic.AC_GameLogic_C|GetPlayerThrusterList (Variables|Default|GetAC_GameLogic)) Index)))

(fn GetPlayerPilot
  (params (Index :type Integer))
  (return (Utilities|Array|Get(acopy) (Variables|/Game/_Added/Utilities/AC_GameLogic.AC_GameLogic_C|GetPlayerPilotList (Variables|Default|GetAC_GameLogic)) Index)))